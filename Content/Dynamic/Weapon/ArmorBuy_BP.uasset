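; ArmorBuy_BP is a world buy point, named for armor, that shows an unlockable's name and cost to nearby players.
; When an FPS_Character_BP enters the TriggerVolume, it adds that character's BuyUIRef widget to the viewport if needed and passes it UnlockableCost and UnlockableName.
; Leaving the volume removes the widget.
; The Blueprint only drives this display and contains no purchase logic.
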(event OnComponentBeginOverlap(TriggerVolume)
  (params (OverlappedComponent :type Primitive%20Component%20Object%20Reference) (OtherActor :type Actor%20Object%20Reference) (OtherComp :type Primitive%20Component%20Object%20Reference) (OtherBodyIndex :type Integer) (bFromSweep :type Boolean) (SweepResult :type Hit%20Result%20Structure%20%28by%20ref%29))
  (bind _asfps_character_bp (Utilities|Casting|CastToFPS_Character_BP OtherActor))
  (if (UserInterface|Viewport|IsinViewport (Variables|/Game/Dynamic/Character/Behaviour/FPS_Character_BP.FPS_Character_BP_C|GetBuy_UI_Ref _asfps_character_bp))
    _
    (else
      (UserInterface|Viewport|AddtoViewport (Variables|/Game/Dynamic/Character/Behaviour/FPS_Character_BP.FPS_Character_BP_C|GetBuy_UI_Ref _asfps_character_bp) 0)))
  (Default|UpdateData1 (Variables|/Game/Dynamic/Character/Behaviour/FPS_Character_BP.FPS_Character_BP_C|GetBuy_UI_Ref _asfps_character_bp) (Variables|Default|GetUnlockableCost) (Variables|Default|GetUnlockableName)))

(event OnComponentEndOverlap(TriggerVolume)
  (params (OverlappedComponent :type Primitive%20Component%20Object%20Reference) (OtherActor :type Actor%20Object%20Reference) (OtherComp :type Primitive%20Component%20Object%20Reference) (OtherBodyIndex :type Integer))
  (bind _asfps_character_bp (Utilities|Casting|CastToFPS_Character_BP OtherActor))
  (Widget|RemovefromParent (Variables|/Game/Dynamic/Character/Behaviour/FPS_Character_BP.FPS_Character_BP_C|GetBuy_UI_Ref _asfps_character_bp)))

(event EventBeginPlay)

(event Collision|EventActorBeginOverlap
  (params (OtherActor :type Actor%20Object%20Reference)))

(event EventTick
  (params (DeltaSeconds :type Float%20%28single-precision%29)))

(fn ConstructionScript)