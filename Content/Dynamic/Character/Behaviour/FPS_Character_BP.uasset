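; First-person character Blueprint that handles the player's HUD, weapon crosshair and sniper scope overlay.
; On BeginPlay it creates the main HUD, weapon-buy and scope widgets, showing only the HUD, then binds weapon-switch and aim-down-sights events.
; Weapon switches refresh the dynamic crosshair.
; Entering ADS with a sniper rifle swaps the HUD for the scope overlay, and exiting restores it.
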(event Custom|ADS%20exit
  (CallFunction|HideSniperScope))

(event Custom|Character%20weapon%20switch
  (Default|UpdateCrosshair (Variables|/Game/Dynamic/UI/MainHUD.MainHUD_C|GetDynamicCrosshair (Variables|Default|GetMainHUD%20ref))))

(event Custom|ADS%20enter
  (CallFunction|ShowSniperScope))

(event EventBeginPlay
  (Utilities|FlowControl|Sequence
    (:then_0
      (CallFunction|CreateWidgets))
    (:then_1
      (EventDispatchers|AssignCharacterWeaponSwitch (delegate Custom|Character%20weapon%20switch)))
    (:then_2
      (EventDispatchers|AssignEventADSEnter (delegate Custom|ADS%20enter)))
    (:then_3
      (EventDispatchers|AssignEventADSExit (delegate Custom|ADS%20exit)))))

(fn ConstructionScript)

(fn CreateWidgets
  (Utilities|FlowControl|Sequence
    (:then_0
      (bind _returnvalue (UserInterface|CreateWidget "/Game/Dynamic/UI/MainHUD.MainHUD_C"))
      (bind _output_get (Variables|Default|SetMainHUD%20ref _returnvalue))
      (UserInterface|Viewport|AddtoViewport _output_get 0))
    (:then_1
      (bind _returnvalue_2 (UserInterface|CreateWidget "/Game/Dynamic/UI/UIWeaponBUy.UIWeaponBUy_C"))
      (Variables|Default|SetWeaponBuy%20ref _returnvalue_2))
    (:then_2
      (bind _returnvalue_3 (UserInterface|CreateWidget "/Game/Dynamic/UI/SniperScope_UI.SniperScope_UI_C"))
      (Variables|Default|SetSniperScope%20ref _returnvalue_3))))

(fn ShowSniperScope
  (bind _sniperscope_ref (Variables|Default|GetSniperScope%20ref))
  (if (Utilities|Enum|Equal(Enum) (Variables|/Script/ProjectZ.WeaponBase|GetWeaponType (Variables|Default|GetCurrentWeapon)) "SniperRifle")
    (Widget|SetVisibility (Variables|Default|GetMainHUD%20ref) "Collapsed")
    (if (not (UserInterface|Viewport|IsinViewport _sniperscope_ref))
      (UserInterface|Viewport|AddtoViewport _sniperscope_ref 0))))

(fn HideSniperScope
  (bind _sniperscope_ref (Variables|Default|GetSniperScope%20ref))
  (if (UserInterface|Viewport|IsinViewport _sniperscope_ref)
    (Widget|SetVisibility (Variables|Default|GetMainHUD%20ref) "Visible")
    (Widget|RemovefromParent _sniperscope_ref)))